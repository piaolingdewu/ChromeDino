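; RandomEntity is a spawner actor that lays out a chain of Entity_BP_Child actors at random spacing along the X axis.
; From BeginPlay, a 0.4-second delay loop counts Maxinterval down, calling SpawnEntity until it reaches zero.
; Each spawn offsets X from LatestLocation by a random MinDistance-to-MaxDistance amount, keeps Y and Z, then stores the new actor's location for the next.
; CheckPlayerLocation is an unused, empty stub.
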(event EventBeginPlay
  (Utilities|FlowControl|Delay 0.4 :!label _label)
  (if (|({506A7AD4-45C6-5A76-A98B-7A9F71685B40}!=0))
    (Math|Integer|DecrementInt (Variables|Default|GetMaxinterval)
      (:%20%20
        (CallFunction|SpawnEntity)
        (goto _label)))))

(event Collision|EventActorBeginOverlap
  (params (OtherActor :type Actor%20Object%20Reference)))

(event EventTick
  (params (DeltaSeconds :type Float%20%28single-precision%29)))

(fn ConstructionScript)

(fn SpawnEntity
  (bind _returnvalue (Game|SpawnActorfromClass "/Game/BluePrint/Entity/Cactaoeae/Entity_BP_Child.Entity_BP_Child_C" (Math|Transform|MakeTransform (Math|Vector|MakeVector (Math|Random|RandomFloatinRange (|({CE0A24D5-4C8C-4F8D-E62D-26B6949B7799}+LatestLocationX) (.X (Math|Vector|BreakVector (Variables|Default|GetLatestLocation)))) (|({9FF3F82F-4416-3535-6484-0B9D7EB9F73F}+LatestLocationX) (.X (Math|Vector|BreakVector (Variables|Default|GetLatestLocation))))) (.Y (Math|Vector|BreakVector (Variables|Default|GetLatestLocation))) (.Z (Math|Vector|BreakVector (Variables|Default|GetLatestLocation))))) "Undefined" 0 0))
  (Variables|Default|SetLatestLocation (Transformation|GetActorLocation _returnvalue)))

(fn CheckPlayerLocation
  (if true
    _))