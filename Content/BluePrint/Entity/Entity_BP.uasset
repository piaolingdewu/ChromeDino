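; Entity Blueprint that reacts to overlaps with the player character DionChar_BP, acting as a one-shot spawn trigger.
; On the first Box overlap with that character, it sets a Spawn flag and calls SpawnEntity on the first RandomEntity_BP found in the level.
; A separate Overlap Event function changes Dion's status when the overlapped component is a Paper flipbook, though this graph never calls it.
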(event OnComponentBeginOverlap(Box)
  (params (OverlappedComponent :type Primitive%20Component%20Object%20Reference) (OtherActor :type Actor%20Object%20Reference) (OtherComp :type Primitive%20Component%20Object%20Reference) (OtherBodyIndex :type Integer) (bFromSweep :type Boolean) (SweepResult :type Hit%20Result%20Structure%20%28by%20ref%29))
  (Utilities|Casting|CastToDionChar_BP OtherActor)
  (if (not (Variables|Default|Getspawn))
    (Variables|Default|Setspawn true)
    (bind _outactors (Actor|GetAllActorsOfClass "/Game/BluePrint/Entity/RandomEntity/RandomEntity_BP.RandomEntity_BP_C"))
    (Default|SpawnEntity (Utilities|Array|Get(acopy) _outactors))))

(event Collision|EventActorBeginOverlap
  (params (OtherActor :type Actor%20Object%20Reference)))

(fn ConstructionScript)

(fn OverlapEvent
  (params (OtherActor :type Actor%20Object%20Reference) (OtherComponent :type Actor%20Component%20Object%20Reference))
  (bind (_asdion_char_bp _bsuccess) (Utilities|Casting|CastToDionChar_BP OtherActor))
  (if _bsuccess
    (if (.bSuccess (Utilities|Casting|CastToPaperFlipbookComponent OtherComponent))
      (Default|ChangeDionStatus _asdion_char_bp "NewEnumerator1"))))