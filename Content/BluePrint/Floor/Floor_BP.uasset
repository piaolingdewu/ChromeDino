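; Floor_BP is a floor segment that spawns the next copy of itself as DionChar_BP advances, extending the floor along world +X.
; When the character begins overlapping the Box1 trigger, SpawnFloor places a new Floor_BP offset by twice the Box X extent from its own location.
; A Spawn flag limits each segment to one successor, and the file contains no cleanup of earlier segments.
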(event OnComponentBeginOverlap(Box1)
  (params (OverlappedComponent :type Primitive%20Component%20Object%20Reference) (OtherActor :type Actor%20Object%20Reference) (OtherComp :type Primitive%20Component%20Object%20Reference) (OtherBodyIndex :type Integer) (bFromSweep :type Boolean) (SweepResult :type Hit%20Result%20Structure%20%28by%20ref%29))
  (Utilities|IsValid (.AsDion%20Char%20BP (Utilities|Casting|CastToDionChar_BP OtherActor))
    (:Is%20Valid
      (CallFunction|SpawnFloor))))

(event OnComponentHit(Box1)
  (params (HitComponent :type Primitive%20Component%20Object%20Reference) (OtherActor :type Actor%20Object%20Reference) (OtherComp :type Primitive%20Component%20Object%20Reference) (NormalImpulse :type Vector :default "0, 0, 0") (Hit :type Hit%20Result%20Structure%20%28by%20ref%29)))

(event EventBeginPlay)

(event Collision|EventActorBeginOverlap
  (params (OtherActor :type Actor%20Object%20Reference)))

(event EventTick
  (params (DeltaSeconds :type Float%20%28single-precision%29)))

(fn ConstructionScript)

(fn SpawnFloor
  (if (not (Variables|Default|Getspawn))
    (Variables|Default|Setspawn true)
    (Game|SpawnActorfromClass "Floor_BP_C" (Math|Transform|MakeTransform (+ (Transformation|GetActorLocation) (Math|Vector|MakeVector (|(a*2) (.X (Math|Vector|BreakVector (Variables|/Script/Engine.BoxComponent|GetBoxExtent (Variables|Default|GetBox))))) 0.0 0.0))) "Undefined" 0 0)))