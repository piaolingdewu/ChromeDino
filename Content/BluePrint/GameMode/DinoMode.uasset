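; DinoMode is a game mode Blueprint for a dino game that raises difficulty over time.
; From BeginPlay, chained one-shot timers step LevelIndex up twice at fixed intervals, printing a difficulty-up message each time.
; GetLevelConst returns the LevelDef entry for the current level.
; A separate InitEvent caches the first RandomEntity_BP actor and the player's DionGameContorll_BP controller.
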(event Custom|Init%20Event
  (CallFunction|InitRandomEntity)
  (CallFunction|InitDinoControll))

(event Custom|Default%20Level
  (Utilities|Time|SetTimerbyEvent (delegate Custom|Level%20Up%20To%201) 6.0))

(event Custom|Level%20Up%20To%201
  (Utilities|Time|SetTimerbyEvent (delegate Custom|Level%20Up%20To%202) 6.0)
  (Variables|Default|SetLevel%20Index 1)
  (Development|PrintString "难度上升"))

(event Custom|Level%20Up%20To%202
  (Variables|Default|SetLevel%20Index 2)
  (Development|PrintString "难度上升"))

(event EventBeginPlay
  (CallFunction|DefaultLevel))

(fn ConstructionScript)

(fn InitRandomEntity
  (bind _outactors (Actor|GetAllActorsOfClass "/Game/BluePrint/Entity/RandomEntity/RandomEntity_BP.RandomEntity_BP_C"))
  (Variables|Default|SetRandomEntity (Utilities|Array|Get(acopy) _outactors)))

(fn InitDinoControll
  (bind _asdion_game_contorll_bp (Utilities|Casting|CastToDionGameContorll_BP (Game|GetPlayerController 0))
    (:then
      (Variables|Default|SetDinoControll _asdion_game_contorll_bp))
    (:CastFailed
      (Development|PrintString "Hello"))))

(fn GetLevelConst
  (return (Utilities|Array|Get(acopy) (Variables|Default|GetLevelDef) (Variables|Default|GetLevel%20Index))))