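; Cloud manager actor that spawns Cloud_BP actors ahead of the player's pawn.
; An endless loop from BeginPlay waits Density seconds, then spawns one at DistanceOfDino ahead on X, with random Y and Z within set ranges.
; DinoMode's dino-death and game-reset events clear and set a SpawnCloud flag, but the spawn loop shown never reads it.
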(event Custom|StartSpawnCloud
  (Variables|Default|SetbSpawnCloud true))

(event Custom|StopSpawnCloud
  (Variables|Default|SetbSpawnCloud false))

(event EventBeginPlay
  (bind _returnvalue (Game|GetGameMode))
  (bind _asdino_mode (Utilities|Casting|CastToDinoMode _returnvalue))
  (EventDispatchers|BindEventtoOnDinoDead _asdino_mode (delegate Custom|StopSpawnCloud))
  (EventDispatchers|BindEventtoOnGameReset _asdino_mode (delegate Custom|StartSpawnCloud))
  (Utilities|FlowControl|Delay (Variables|Default|Getdensity) :!label _label)
  (CallFunction|SpawnCloud)
  (goto _label))

(event Collision|EventActorBeginOverlap
  (params (OtherActor :type Actor%20Object%20Reference)))

(event EventTick
  (params (DeltaSeconds :type Float%20%28single-precision%29)))

(fn ConstructionScript)

(fn SpawnCloud
  (Game|SpawnActorfromClass "/Game/BluePrint/could/Cloud_BP.Cloud_BP_C" (Math|Transform|MakeTransform (Math|Vector|MakeVector (+ (Variables|Default|GetDistanceOfDino) (.X (Math|Vector|BreakVector (Transformation|GetActorLocation (Game|Player|GetPlayerPawn 0))))) (Math|Random|RandomFloatinRange (Variables|Default|GetMinY) (Variables|Default|GetMaxY)) (Math|Random|RandomFloatinRange (Variables|Default|GetMinZ) (Variables|Default|GetMaxZ)))) "Undefined" 0 0))