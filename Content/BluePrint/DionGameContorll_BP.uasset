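; DionGameContorll_BP is the player controller for a dino game, handling the cursor, camera view and game status.
; It shows the mouse cursor on BeginPlay, and on possess it calls PossessDino and switches the view target to the DinoCamera_BP actor.
; Helper functions get and set GameStatus and expose the camera and its location, taking the first DinoCamera_BP found by GetAllActorsOfClass on each call.
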(event EventPossess
  (params (PossessedPawn :type Pawn%20Object%20Reference))
  (Default|CallPossessDino)
  (Game|Player|SetViewTargetwithBlend (CallFunction|GetDionCamera) 0.0 "VTBlend_Linear" 0.0 false))

(event EventTick
  (params (DeltaSeconds :type Float%20%28single-precision%29)))

(event EventBeginPlay
  (Variables|Default|SetbShowMouseCursor true))

(fn ConstructionScript)

(fn GetGameStatus
  (return (Variables|Default|GetGameStatus)))

(fn SetGameStatus
  (params (GameStatus :type GameStatus%20Enum :default "NewEnumerator0"))
  (Variables|Default|SetGameStatus GameStatus))

(fn GetDionCameraLocation
  (return (Transformation|GetActorLocation (CallFunction|GetDionCamera))))

(fn GetDionCamera
  (bind _outactors (Actor|GetAllActorsOfClass "/Game/BluePrint/Dion/DinoCamera_BP.DinoCamera_BP_C"))
  (return (Utilities|Array|Get(acopy) _outactors)))