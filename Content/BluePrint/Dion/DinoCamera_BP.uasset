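; DinoCamera_BP is a camera actor that follows the player-controlled pawn along the world X axis.
; Each Tick it feeds the pawn's X, with Y and Z zeroed, into a PawnLocation + Rellocation math expression and moves itself to the result.
; The nodes deriving Rellocation from the first DionChar_BP are disconnected, so that offset is never computed here.
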(event EventBeginPlay)

(event Collision|EventActorBeginOverlap
  (params (OtherActor :type Actor%20Object%20Reference)))

(event EventTick
  (params (DeltaSeconds :type Float%20%28single-precision%29))
  (Transformation|SetActorLocation (|(PawnLocation+{B88B9145-458F-F475-8500-178411EDAA08}) (Math|Vector|MakeVector (.X (Math|Vector|BreakVector (Transformation|GetActorLocation (Pawn|GetControlledPawn (Game|GetPlayerController 0))))) 0.0 0.0)) false false))

(fn ConstructionScript)