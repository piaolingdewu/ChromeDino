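; Player character for a side-view endless-runner style game: a flipbook-animated Dion that auto-runs along +X and jumps on Space.
; ChangeDionStatus drives a Wait, Runing and Dead state machine, swapping flipbooks; floor hits resume running.
; Holding Space lowers gravity scale for higher jumps.
; Death, triggered here by the E key, stops movement and input, then spawns GameOver_BP relative to the controller's camera location.
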(event OnComponentHit(CapsuleComponent)
  (params (HitComponent :type Primitive%20Component%20Object%20Reference) (OtherActor :type Actor%20Object%20Reference) (OtherComp :type Primitive%20Component%20Object%20Reference) (NormalImpulse :type Vector :default "0, 0, 0") (Hit :type Hit%20Result%20Structure%20%28by%20ref%29))
  (if (|((a==b)==c) (.bSuccess (Utilities|Casting|CastToFloor_BP OtherActor)) (Utilities|Enum|NotEqual(Enum) (Variables|Default|GetStatus) "NewEnumerator1") true)
    (CallFunction|ChangeDionStatus "NewEnumerator2")))

(event EventBeginPlay
  (CallFunction|ChangeDionStatus "NewEnumerator2"))

(event Collision|EventActorBeginOverlap
  (params (OtherActor :type Actor%20Object%20Reference)))

(event EventTick
  (params (DeltaSeconds :type Float%20%28single-precision%29))
  (Utilities|FlowControl|Sequence
    (:then_1
      (if (Utilities|Enum|Equal(Enum) (Variables|Default|GetStatus) "NewEnumerator2")
        (Class|PawnMovementComponent|AddInputVector (Variables|Character|GetCharacterMovement) "1.000000, 0, 0" false)))))

(event Input|AxisEvents|InputAxisJump
  (params (AxisValue :type Float%20%28single-precision%29)))

(event Input|KeyboardEvents|E
  (params (Key :type Key%20Structure))
  (:Pressed
    (CallFunction|ChangeDionStatus "NewEnumerator1")))

(event Input|KeyboardEvents|SpaceBar
  (params (Key :type Key%20Structure))
  (bind _charactermovement (Variables|Character|GetCharacterMovement))
  (:Pressed
    (Variables|/Script/Engine.CharacterMovementComponent|SetGravityScale _charactermovement 2.4)
    (Character|Jump)
    (CallFunction|ChangeDionStatus "NewEnumerator0"))
  (:Released
    (Variables|/Script/Engine.CharacterMovementComponent|SetGravityScale _charactermovement 4.0)))

(fn ConstructionScript
  (CallFunction|ChangeDionStatus "NewEnumerator0"))

(fn ChangeDionStatus
  (params (Selection :type DionStatus%20Enum :default "NewEnumerator0"))
  (bind _charactermovement (Variables|Character|GetCharacterMovement))
  (bind _sprite (Variables|Default|GetSprite))
  (bind _output_get (Variables|Default|SetStatus Selection))
  (switch Utilities|FlowControl|Switch|SwitchonDionStatus _output_get
    (:NewEnumerator0
      (Sprite|SetFlipbook _sprite "/Game/BluePrint/Dion/Animation/DionWait.DionWait"))
    (:NewEnumerator1
      (Variables|/Script/Engine.CharacterMovementComponent|SetGravityScale _charactermovement 0.0)
      (Components|Movement|StopMovementImmediately _charactermovement)
      (Input|DisableInput self 0)
      (Sprite|SetFlipbook _sprite "/Game/BluePrint/Dion/Animation/DionDead.DionDead")
      (Game|SpawnActorfromClass "/Game/BluePrint/UI/GameOver_BP.GameOver_BP_C" (Math|Transform|MakeTransform (- (Default|GetDionCameraLocation (.AsDion%20Game%20Contorll%20BP (Utilities|Casting|CastToDionGameContorll_BP (Pawn|GetController self)))) "0,300.000000, 0")) "Undefined" 0 0))
    (:NewEnumerator2
      (Sprite|SetFlipbook _sprite "/Game/BluePrint/Dion/Animation/DionRuning.DionRuning"))))